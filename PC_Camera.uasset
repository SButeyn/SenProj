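; PC_Camera is a player controller Blueprint that handles mouse-driven tower placement and its resource cost.
; While placing, Tick moves a ghost actor to the deprojected mouse world location flattened to zero height, without a trace.
; Releasing left mouse, if placement is allowed, spawns the tower there, destroys the ghost, exits placement and deducts a fixed cost.
; Nothing here starts placement, creates the ghost, updates validity or checks affordability.
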(event `self.ReceiveBeginPlay`
  (set `self.placing tower` false)
  (set `self.can place` true))

(event `self.ReceiveTick`
  (params (DeltaSeconds :type "Float (single-precision)"))
  (if (`self.placing tower`)
    (set `self.holdVector` (`KismetMathLibrary.MakeVector` (.x (`self.DeprojectMousePositionToWorld`)) (.y (`self.DeprojectMousePositionToWorld`))))
    (`self.K2_SetActorLocation` (`self.ghost`) (`self.holdVector`) false false)))

(event `Key|LeftMouseButton`
  (params (Key :type "Key Structure" :default "AnyKey"))
  (:`Released`
    (if (`self.placing tower`)
      (if (`self.can place`)
        (`|SpawnActorFromClass` "/Game/MyTower.MyTower_C" (`KismetMathLibrary.MakeTransform` (`self.holdVector`)) "Undefined" "OverrideRootScale")
        (set `self.placing tower` false)
        (`self.K2_DestroyActor` (`self.ghost`))
        (set `self.int_resources` (- (`self.int_resources`) 100))))))

(fn `UserConstructionScript`)